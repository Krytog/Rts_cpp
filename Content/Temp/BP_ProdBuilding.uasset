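; BP_ProdBuilding is a building Blueprint in a Temp folder that shows an arrow pointing at a target actor, apparently as a prototype.
; On BeginPlay it aims the ArrowToTaget component at Target's location and makes it visible.
; Pressing E re-aims the arrow at the location of the actor under the cursor, found by a complex Visibility trace, with debug prints for the key press and invalid hits.
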(event EventBeginPlay
  (bind _arrowtotaget (Variables|Default|GetArrowToTaget))
  (Class|ArrowtoTagetComponent|SetTargetLocation _arrowtotaget (Transformation|GetActorLocation (Variables|Default|GetTarget)))
  (Class|ArrowtoTagetComponent|SetArrowVisibility _arrowtotaget true))

(event Input|KeyboardEvents|E
  (params (Key :type Key%20Structure :default "None"))
  (bind _returnvalue (Game|GetPlayerController 0))
  (bind _arrowtotaget (Variables|Default|GetArrowToTaget))
  (bind _hitresult (Game|Player|GetHitResultUnderCursorbyChannel _returnvalue "TraceTypeQuery1" true))
  (bind _hitactor (Collision|BreakHitResult _hitresult))
  (:Pressed
    (Development|PrintString "triggered!" true true "(R=1.000000,G=0.000000,B=0.091857,A=1.000000)")
    (Utilities|IsValid _hitactor
      (:Is%20Valid
        (Class|ArrowtoTagetComponent|SetTargetLocation _arrowtotaget (Transformation|GetActorLocation _hitactor))
        (Class|ArrowtoTagetComponent|SetArrowVisibility _arrowtotaget true))
      (:Is%20Not%20Valid
        (Development|PrintString "BAD ACTOR!")))))

(fn ConstructionScript)