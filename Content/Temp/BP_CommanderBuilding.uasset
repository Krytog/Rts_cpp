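; BP_CommanderBuilding is an actor Blueprint for a commander building that links itself to the player and shows its name on an info widget.
; On BeginPlay it casts player pawn 0 to DefaultPlayer, binds to it, and writes GetInfoName into the WB_Info widget component.
; After a one-second delay it registers itself on that player's minimap.
; A failed cast to the pawn or widget stops the remaining setup.
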(event EventBeginPlay
  (bind _self self)
  (bind _asdefault_player (Utilities|Casting|CastToDefaultPlayer (Game|Player|GetPlayerPawn 0)))
  (Class|Building|BindtoPlayer _asdefault_player)
  (bind _aswb_info (Utilities|Casting|CastToWB_Info (UserInterface|GetWidget (Variables|Default|GetInfoWidgetComponent))))
  (Variables|/Script/UMG.TextBlock|SetText (Variables|/Game/Temp/WB_Info.WB_Info_C|GetInfoName _aswb_info) (Class|Building|GetInfoName _self))
  (Utilities|FlowControl|Delay 1.0)
  (Class|Unit|RegisteronMinimap _self _asdefault_player))

(fn ConstructionScript)